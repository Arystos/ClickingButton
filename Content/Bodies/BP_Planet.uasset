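; BP_Planet is a celestial body that randomizes itself at spawn and explodes on collision with another planet or a star.
; BeginPlay applies a random texture through a dynamic material, rolls Mass to drive clamped mesh scale, and picks a random XY InitialVelocity if none is set.
; On a hit it spawns a Niagara burst aimed against its Velocity, then destroys itself.
; No movement or gravity logic appears in these graphs.
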(event `self.ReceiveBeginPlay`
  (bind _returnvalue (`KismetMathLibrary.RandomFloatInRange` 100.0 250.0))
  (bind _bodymesh (`self.BodyMesh`))
  (`|ExecutionSequence`
    (:`then_0`
      (`/Engine/EditorBlueprintResources/StandardMacros.IsValid` (`self.BodyMesh`)
        (:`Is Valid`
          ;[1 1 1] Random Planet Proprieties
          (bind _returnvalue_2 (`PrimitiveComponent.CreateDynamicMaterialInstance` _bodymesh 0 (`PrimitiveComponent.GetMaterial` _bodymesh 0) "None"))
          (`MaterialInstanceDynamic.SetTextureParameterValue` _returnvalue_2 "PlanetTexture" (`KismetArrayLibrary.Array_Random` (`self.Value`))))
        (:`Is Not Valid`
          (`KismetSystemLibrary.PrintString` "Material not valid")))
      (bind _output_get (set `self.Mass` (`KismetMathLibrary.RandomFloatInRange` 100.0 400.0)))
      (`SceneComponent.SetRelativeScale3D` (`self.BodyMesh`) (`KismetMathLibrary.Conv_DoubleToVector` (/ (`KismetMathLibrary.FClamp` _output_get 50.0 200.0) 200.0))))
    (:`then_1`
      ;[1 1 1] Randomize Rotation and Velocity
      (if (not (!= (`self.InitialVelocity`) (0.0 0.0 0.0)))
        (set `self.InitialVelocity` (`KismetMathLibrary.MakeVector` _returnvalue _returnvalue))))))

(event `self.BodyMesh.OnComponentHit`
  (params (HitComponent :type "PrimitiveComponent Object Reference") (OtherActor :type "Actor Object Reference") (OtherComp :type "PrimitiveComponent Object Reference") (NormalImpulse :type "Vector Structure") (Hit :type "HitResult Structure (by ref)"))
  (bind _returnvalue (`GameplayStatics.GetObjectClass` OtherActor))
  (if (or (== _returnvalue "BP_Planet_C") (== _returnvalue "/Game/Bodies/BP_Star.BP_Star_C"))
    ;[1 1 1] Niagara Burst Proprieties
    (bind _returnvalue_2 (`NiagaraFunctionLibrary.SpawnSystemAtLocation` "/Game/Bodies/NS_CollisionBurst.NS_CollisionBurst" (`self.K2_GetActorLocation`)))
    (`FXSystemComponent.SetFloatParameter` _returnvalue_2 "Core Burst size" (`self.Burst Core Size`))
    (`FXSystemComponent.SetVectorParameter` _returnvalue_2 "Velocity" (* (* (`KismetMathLibrary.Normal` (`self.Velocity`)) -1.0) (`self.Burst FOrce`)))
    (`FXSystemComponent.SetIntParameter` _returnvalue_2 "Burst Amount" (`self.Burst Amount`))
    (set `self.Velocity` (0.0 0.0 0.0))
    (`self.K2_DestroyActor`)))

(fn `UserConstructionScript`)