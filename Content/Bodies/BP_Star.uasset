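; BP_Star is a star body with a mesh and point light that bursts when it collides with another star.
; On BeginPlay, a zero InitialVelocity triggers a random XY velocity and a random palette color, applied to the light and a dynamic material unless pure white.
; On a hit with another BP_Star, it spawns a tuned Niagara burst at their midpoint and destroys both actors.
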(event `self.ReceiveBeginPlay`
  (bind _returnvalue (`KismetMathLibrary.RandomFloatInRange` 1.0 5.0))
  (bind _bodymesh (`self.BodyMesh`))
  (bind _star_color (`self.Star Color`))
  ;[1 1 1] Initialize velocity
  (if (not (!= (`self.InitialVelocity`) (0.0 0.0 0.0)))
    (set `self.InitialVelocity` (`KismetMathLibrary.MakeVector` _returnvalue _returnvalue))
    ;[1 1 1] Generate Star Color
    (bind _returnvalue_2 (`PrimitiveComponent.CreateDynamicMaterialInstance` _bodymesh 0 (`PrimitiveComponent.GetMaterial` _bodymesh 0) "None"))
    (bind _output_get (set `self.Star Color` (`KismetArrayLibrary.Array_Random` (`self.Color Array`))))
    (bind (_b _g _r) (break `Color` _output_get))
    ;;[1 1 1] If pure white don't change the standard color
    (if (not (`KismetMathLibrary.EqualExactly_VectorVector` (`KismetMathLibrary.MakeVector` (`KismetMathLibrary.Conv_ByteToDouble` _b) (`KismetMathLibrary.Conv_ByteToDouble` _g) (`KismetMathLibrary.Conv_ByteToDouble` _r)) (255.0 255.0 255.0)))
      ;;[1 1 1] Create another star color
      (`LightComponent.SetLightColor` (`self.PointLight`) (`KismetMathLibrary.Conv_ColorToLinearColor` _star_color) true)
      (`MaterialInstanceDynamic.SetVectorParameterValue` _returnvalue_2 "Color" (`KismetMathLibrary.Conv_ColorToLinearColor` _star_color)))))

(event `self.BodyMesh.OnComponentHit`
  (params (HitComponent :type "PrimitiveComponent Object Reference") (OtherActor :type "Actor Object Reference") (OtherComp :type "PrimitiveComponent Object Reference") (NormalImpulse :type "Vector Structure") (Hit :type "HitResult Structure (by ref)"))
  (if (== (`GameplayStatics.GetObjectClass` OtherActor) "BP_Star_C")
    (bind _returnvalue (`NiagaraFunctionLibrary.SpawnSystemAtLocation` "/Game/Bodies/NS_CollisionBurst.NS_CollisionBurst" (/ (+ (`self.K2_GetActorLocation` OtherActor) (`self.K2_GetActorLocation`)) 2)))
    (set `self.Burst Niagara` _returnvalue)
    (`FXSystemComponent.SetFloatParameter` (`self.Burst Niagara`) "Intensity" 10000.0)
    (`FXSystemComponent.SetFloatParameter` (`self.Burst Niagara`) "Core Burst size" (`self.Burst Core Size`))
    (`FXSystemComponent.SetIntParameter` (`self.Burst Niagara`) "Burst Amount" 500)
    (`FXSystemComponent.SetFloatParameter` (`self.Burst Niagara`) "Sparkle Lifetime" 3.0)
    (`FXSystemComponent.SetFloatParameter` (`self.Burst Niagara`) "Core Lifetime" 6.0)
    (`self.K2_DestroyActor` OtherActor)
    (`self.K2_DestroyActor`)))

(fn `UserConstructionScript`)