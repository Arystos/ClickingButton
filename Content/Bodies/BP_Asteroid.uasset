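; BP_Asteroid is an asteroid body that shatters in a particle burst on its first collision.
; On BeginPlay, a zero InitialVelocity is replaced with random positive X and Y speeds, keeping motion in the horizontal plane.
; A DoOnce-guarded mesh hit spawns the NS_CollisionBurst Niagara system, scaling intensity by clamped Mass and aiming the burst opposite Velocity.
; The hit then zeroes Velocity and destroys the actor.
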(event `self.ReceiveBeginPlay`
  (bind _returnvalue (`KismetMathLibrary.RandomFloatInRange` 150.0 350.0))
  (`|ExecutionSequence`
    (:`then_0`
      (if (not (!= (`self.InitialVelocity`) (0.0 0.0 0.0)))
        (set `self.InitialVelocity` (`KismetMathLibrary.MakeVector` _returnvalue _returnvalue))))))

(event `self.BodyMesh.OnComponentHit`
  (params (HitComponent :type "PrimitiveComponent Object Reference") (OtherActor :type "Actor Object Reference") (OtherComp :type "PrimitiveComponent Object Reference") (NormalImpulse :type "Vector Structure") (Hit :type "HitResult Structure (by ref)"))
  (`/Engine/EditorBlueprintResources/StandardMacros.DoOnce` false
    (:`Completed`
      (bind _returnvalue (`NiagaraFunctionLibrary.SpawnSystemAtLocation` "/Game/Bodies/NS_CollisionBurst.NS_CollisionBurst" (`self.K2_GetActorLocation`)))
      (`FXSystemComponent.SetFloatParameter` _returnvalue "Intensity" (`KismetMathLibrary.FClamp` (* (`self.Mass`) 1000.0) 10.0 10000.0))
      (`FXSystemComponent.SetVectorParameter` _returnvalue "Velocity" (* (* (`KismetMathLibrary.Normal` (`self.Velocity`)) -1.0) (`self.Burst FOrce`)))
      (`FXSystemComponent.SetFloatParameter` _returnvalue "Core Burst size" (`self.Burst Core Size`))
      (`FXSystemComponent.SetFloatParameter` _returnvalue "Burst Amount" 20.0)
      (set `self.Velocity` (0.0 0.0 0.0))
      (`self.K2_DestroyActor`))))

(fn `UserConstructionScript`)