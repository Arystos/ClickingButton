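; Interactable button that spawns a celestial body: an asteroid, planet or star.
; A looping timer cycles the selected body and updates the text label.
; On interact it briefly plays the press animation and a sound, then spawns the selected class at a random location around the world origin and resets to asteroid.
; A game mode call to refill the bodies array is present but disconnected.
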(event `self.ReceiveBeginPlay`
  (`self.SetSpawnText` "Asteroid")
  (`KismetSystemLibrary.K2_SetTimerDelegate` (delegate `Change Body to Spawn`) 5.0 true))

(event `Change Body to Spawn`
  (bind _body_to_spawn (`self.Body To Spawn`))
  (`/Engine/EditorBlueprintResources/StandardMacros.IncrementInt` _body_to_spawn
    (:`  `
      (bind _output_get (set `self.Body To Spawn` (mod _body_to_spawn 3)))
      (switch `int` _output_get
        (:`0`
          (`self.SetSpawnText` "Asteroid"))
        (:`1`
          (`self.SetSpawnText` "Planet"))
        (:`2`
          (`self.SetSpawnText` "Star"))))))

(event `/Game/Button/BPI_Interactable.OnInteract`
  (params (InteractingPlayer :type "Character Object Reference"))
  (bind _spawnrange (`self.SpawnRange`))
  (bind _returnvalue (* _spawnrange -1.0))
  (bind _asbp_anim_button (cast `/Game/Player/Button/BP_Anim_Button` (`SkeletalMeshComponent.GetAnimInstance` (`self.ButtonMesh`))))
  (set `/Game/Player/Button/BP_Anim_Button.IsPressed` true _asbp_anim_button)
  (`AudioComponent.Play` (`self.Audio`) 0.0)
  (`KismetSystemLibrary.Delay` 0.2)
  (set `/Game/Player/Button/BP_Anim_Button.IsPressed` false _asbp_anim_button)
  (`|SpawnActorFromClass` (`|GetArrayItem` (`self.Bodies Array`) (`self.Body To Spawn`)) (`KismetMathLibrary.MakeTransform` (`KismetMathLibrary.MakeVector` (`KismetMathLibrary.RandomFloatInRange` _returnvalue _spawnrange) (`KismetMathLibrary.RandomFloatInRange` _returnvalue _spawnrange) (`KismetMathLibrary.RandomFloatInRange` 100.0 500.0))) "Undefined" "MultiplyWithRoot" null null)
  (set `self.Body To Spawn` 0)
  (`self.SetSpawnText` "Asteroid"))

(fn `SetSpawnText`
  (params (`Text to Spawn` :type String))
  (`TextRenderComponent.K2_SetText` (`self.TextRender`) (`KismetTextLibrary.Conv_StringToText` (`KismetSystemLibrary.MakeLiteralString` (`KismetStringLibrary.Concat_StrStr` "Spawn a " `Text to Spawn`)))))

(fn `UserConstructionScript`)